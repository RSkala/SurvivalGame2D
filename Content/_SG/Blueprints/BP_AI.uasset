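; BP_AI is a base AI enemy with a Paper2D flipbook that takes hits through an interface event.
; Hits from causers that pass an alive check reduce HP and call HPDisplay, an empty hook for child classes.
; Surviving enemies are launched away from the damage causer by force divided by mass and briefly tinted, with a timer restoring the color.
; Death only prints a debug message; Dead is never set here.
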(event `/Game/_SG/Blueprints/Interfaces/BPI_Combat.INT_HitHandle`
  (params (DamageCauser :type "Actor Object Reference") (Damage :type "Float (double-precision)") (Force :type Integer))
  ;[1 1 1] Hit & Death
  (set `self.Damage Causer` DamageCauser)
  (set `self.ReceivedDamage` Damage)
  (set `self.ReceivedForce` Force)
  (bind _damage_causer (`self.Damage Causer`)
    (:`then`
      (bind _live_ (message `/Game/_SG/Blueprints/Interfaces/BPI_Combat.INT_GetDead` _damage_causer))
      (if (and _live_ (not (`self.Dead`)))
        (bind _output_get (set `self.CurrentHP` (- (`self.CurrentHP`) (`self.ReceivedDamage`))))
        (`self.HPDisplay` _output_get)
        (if (<= _output_get 0.0)
          (`KismetSystemLibrary.PrintString` "DEATH" true true (struct :`R` 1.0 :`G` 0.160202 :`A` 1.0) 0.0)
          (else
            (`self.HandleKnockbackAndColor` (`self.Damage Causer`) (`self.ReceivedForce`))))))
    (:`else`)))

(event `HPDisplay`
  (params (Value :type "Float (double-precision)"))
  ;[1 1 1] Hit & Death
)

(fn `HandleKnockbackAndColor`
  (params (DamageCauser :type "Actor Object Reference") (ReceivedForce :type Integer))
  (`/Engine/EditorBlueprintResources/StandardMacros.IsValid` DamageCauser
    (:`Is Valid`
      (if (!= ReceivedForce 0)
        ;[1 1 1] Handle Knockback - Skip if ReceivedForce is 0
        (`MovementComponent.StopMovementImmediately` (`self.CharacterMovement`))
        (`self.LaunchCharacter` (* (/ ReceivedForce (`self.InfoMass`)) (`KismetMathLibrary.GetDirectionUnitVector` (`self.K2_GetActorLocation` DamageCauser) (`self.K2_GetActorLocation`))) true true)
        (`PaperFlipbookComponent.SetSpriteColor` (`self.PaperFlipbook`) (struct :`R` 1.0 :`G` 0.055509 :`B` 0.518187 :`A` 1.0)))
      (`KismetSystemLibrary.K2_SetTimer` null "ResetColorAndMovement" 0.2))))

(fn `INT_GetDead`
  (returns (`Live?` :type Boolean))
  (return (not (`self.Dead`))))

(fn `ResetColorAndMovement`
  (`KismetSystemLibrary.PrintString` "ResetColorAndMovement")
  ;[1 1 1] Reset the sprite color to White
  (`PaperFlipbookComponent.SetSpriteColor` (`self.PaperFlipbook`) (struct :`R` 1.0 :`G` 1.0 :`B` 1.0 :`A` 1.0)))

(fn `UserConstructionScript`)