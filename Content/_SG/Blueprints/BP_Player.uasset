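; Player character for a top-down Paper2D shooter, moved with Enhanced Input and auto-firing bullets toward the mouse cursor.
; BeginPlay adds the input mapping, sets the idle-down animation and starts a looping fire timer.
; Movement, guarded by a death check, picks directional flipbooks by map key, using two Gates to arbitrate axes; release selects idle from MoveState.
; Key 1 spawns and possesses a spectator pawn linked to the player.
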(event `self.ReceiveBeginPlay`
  ;[1 1 1] BeginPlay
  (`self.Initialization`))

(event `EnhancedInput|/Game/_SG/Inputs/IA_Movement`
  (params (ActionValue :type "Vector2D Structure") (ElapsedSeconds :type "Float (double-precision)") (TriggeredSeconds :type "Float (double-precision)") (InputAction :type "InputAction Object Reference" :default "/Game/_SG/Inputs/IA_Movement.IA_Movement"))
  (bind (_x _y) (`KismetMathLibrary.BreakVector2D` ActionValue))
  (bind _actionvaly (`self.ActionValY`))
  (bind _actionvalx (`self.ActionValX`))
  (bind _returnvalue (> _actionvalx 0.0))
  (bind _returnvalue_2 (> _actionvaly 0.0))
  ;[1 1 1] Player Movement
  (:`Triggered`
    (`self.GeneralCheck`
      (:`true`
        (set `self.ActionValX` _x)
        (set `self.ActionValY` _y)
        (`self.AddMovementInput` (1.0 0.0 0.0) (`self.ActionValX`))
        (`self.AddMovementInput` (0.0 1.0 0.0) (`self.ActionValY`))
        (`|ExecutionSequence`
          (:`then_0`
            (if (!= _actionvaly 0.0)
              (set `self.MoveState` (select `bool` _returnvalue_2 :`false` "NewEnumerator0" :`true` "NewEnumerator1" :!type "/Game/_SG/Blueprints/Enumerations/E_MoveState Enum"))
              (`/Engine/EditorBlueprintResources/StandardMacros.Gate` true :!label _label
                (:`Exit`
                  (`PaperFlipbookComponent.SetFlipbook` (`self.PaperFlipbook`) (select `bool` _returnvalue_2 :`false` (`self.GetProperAnim` "move_up") :`true` (`self.GetProperAnim` "move_down")))
                  (goto _label_2 :!via `Close`)))
              (else
                (goto _label_2 :!via `Open`))))
          (:`then_1`
            (if (!= _actionvalx 0.0)
              (set `self.MoveState` (select `bool` _returnvalue :`false` "NewEnumerator2" :`true` "NewEnumerator3" :!type "/Game/_SG/Blueprints/Enumerations/E_MoveState Enum"))
              (`/Engine/EditorBlueprintResources/StandardMacros.Gate` true :!label _label_2
                (:`Exit`
                  (`PaperFlipbookComponent.SetFlipbook` (`self.PaperFlipbook`) (select `bool` _returnvalue :`false` (`self.GetProperAnim` "move_left") :`true` (`self.GetProperAnim` "move_right")))
                  (goto _label :!via `Close`)))
              (else
                (goto _label :!via `Open`))))))))
  (:`Completed`
    (`PaperFlipbookComponent.SetFlipbook` (`self.PaperFlipbook`) (select `/Game/_SG/Blueprints/Enumerations/E_MoveState` (`self.MoveState`) :`NewEnumerator0` (`self.GetProperAnim` "idle_up") :`NewEnumerator1` (`self.GetProperAnim` "idle_down") :`NewEnumerator2` (`self.GetProperAnim` "idle_left") :`NewEnumerator3` (`self.GetProperAnim` "idle_right")) :!label _label_3)))

(event `InitializeCharacterAnim`
  ;[1 1 1] Player Movement
  (set `self.MoveState` "NewEnumerator1")
  (goto _label_3))

(event `Key|One`
  (params (Key :type "Key Structure"))
  ;[1 1 1] Spectator
  (:`Pressed`
    (bind _returnvalue (`|SpawnActorFromClass` "/Game/_SG/Blueprints/BP_Spectator.BP_Spectator_C" (`self.GetTransform`) "AlwaysSpawn" "MultiplyWithRoot" null null))
    (`Controller.Possess` (`GameplayStatics.GetPlayerController` 0) _returnvalue)
    (set `/Game/_SG/Blueprints/BP_Spectator.PlayerPawn` self _returnvalue)))

(fn `GetProperAnim`
  (params (Str :type String))
  (returns (Anim :type "PaperFlipbook Object Reference"))
  (return (`BlueprintMapLibrary.Map_Find` (`self.CharacterAnimations`) Str)))

(fn `Initialization`
  (bind _aspc_in_game (cast `/Game/_SG/Data/PC_InGame` (`self.GetController`)))
  (bind _returnvalue (pcsubsystem `EnhancedInputLocalPlayerSubsystem` _aspc_in_game))
  (`/Engine/EditorBlueprintResources/StandardMacros.IsValid` _returnvalue
    (:`Is Valid`
      (`EnhancedInputSubsystemInterface.AddMappingContext` _returnvalue "/Game/_SG/Inputs/IMC_SG.IMC_SG" 0 (struct))
      (`self.InitializeCharacterAnim`)
      ;[1 1 1] Repeat AutomaticFiring every X seconds
      (`KismetSystemLibrary.K2_SetTimer` null "temp_AutomaticFiring" 0.7 true))))

(fn `temp_AutomaticFiring`
  (bind (_returnvalue_x _returnvalue_y _returnvalue_z) (`KismetMathLibrary.BreakVector` (`self.K2_GetActorLocation`)))
  (bind (_returnvalue_roll _returnvalue_pitch _returnvalue_yaw) (`KismetMathLibrary.BreakRotator` (`KismetMathLibrary.FindLookAtRotation` (`self.K2_GetActorLocation`) (`PlayerController.DeprojectMousePositionToWorld` (`GameplayStatics.GetPlayerController` 0)))))
  (`|SpawnActorFromClass` "/Game/_SG/Blueprints/BPA/BPA_Bullet.BPA_Bullet_C" (`KismetMathLibrary.MakeTransform` (`KismetMathLibrary.MakeVector` _returnvalue_x _returnvalue_y (- _returnvalue_z 2.0))) "AdjustIfPossibleButAlwaysSpawn" "MultiplyWithRoot" null "enemy" (* (`KismetMathLibrary.Conv_RotatorToVector` (`KismetMathLibrary.MakeRotator` 0.0 0.0 _returnvalue_yaw)) (`self.AtkVel`)) null))

(fn `UserConstructionScript`)