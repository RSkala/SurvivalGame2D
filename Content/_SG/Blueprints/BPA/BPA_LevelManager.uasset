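; BPA_LevelManager is the level manager actor that registers itself on the game instance at BeginPlay and owns the bullet pool.
; PoolingBullet reuses the first pooled bullet in an available state, or spawns a BPA_Bullet at the pool location and adds it.
; It then applies the caller's bullet properties and moves the bullet to the player's location, leaving the Location input unused.
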(event `self.ReceiveBeginPlay`
  (set `/Game/_SG/Data/GI_SG.Ref_LevelManager` self (`/Game/_SG/Data/BPFL_SG.GetSGGameInstance`)))

(fn `PoolingBullet`
  (params (Location :type "Vector Structure") (OverallScale :type "Vector Structure") (Damage :type "Float (double-precision)") (ProjectileVelocity :type "Vector Structure") (TargetTag :type Name) (DamageCauser :type "Actor Object Reference") (NewFlipbook :type "PaperFlipbook Object Reference") (FlipbookScale :type "Vector Structure") (LifeSpan :type "Float (double-precision)"))
  (locals (L_AvailableBullet :type "/Game/_SG/Blueprints/BPA/BPA_Bullet Object Reference"))
  (bind _l_availablebullet (`local.L_AvailableBullet`))
  (for _array_element (`self.BulletPool`)
    (if (`|EnumEquality` (`/Game/_SG/Blueprints/BPA/BPA_Bullet.BulletState` _array_element) "NewEnumerator1")
      ;[1 1 1] Found available bullet in pool
      (set `local.L_AvailableBullet` _array_element)
      (break)))
  (`local.L_AvailableBullet`
    (:`then`
      _)
    (:`else`
      ;[1 1 1] If L_AvailableBullet is not valid, then NO available bullets were found in the BulletPool. Create a new bullet
      (bind _returnvalue (`|SpawnActorFromClass` "/Game/_SG/Blueprints/BPA/BPA_Bullet.BPA_Bullet_C" (`KismetMathLibrary.MakeTransform` (`self.BulletPoolLocation`)) "AdjustIfPossibleButAlwaysSpawn" "MultiplyWithRoot" null "None" (0.0 0.0 0.0) null))
      ;[1 1 1] Add the newly created bullet into the BulletPool
      (bind _output_get (set `local.L_AvailableBullet` _returnvalue))
      (`KismetArrayLibrary.Array_Add` (`self.BulletPool`) _output_get)))
  ;[1 1 1] Set up bullet properties on the newly active bullet
  (`/Game/_SG/Blueprints/BPA/BPA_Bullet.SetupBulletProperties` _l_availablebullet (`local.OverallScale`) (`local.Damage`) (`local.ProjectileVelocity`) (`local.TargetTag`) (`local.DamageCauser`) (`local.NewFlipbook`) (`local.FlipbookScale`) (`local.LifeSpan`))
  ;[1 1 1] Set the bullet's position at the player character's position
  (`self.K2_SetActorLocation` _l_availablebullet (`self.K2_GetActorLocation` (`/Game/_SG/Data/GI_SG.Ref_Player` (`/Game/_SG/Data/BPFL_SG.GetSGGameInstance`))) false false))

(fn `UserConstructionScript`)